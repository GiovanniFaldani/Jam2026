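; Game mode for a card game that runs a turn state machine, of which only the Refresh state is implemented.
; BeginPlay gathers every BP_DummyCard actor into a shuffled deck and sets the state to Refresh.
; Tick uses a done flag to run refresh, then advances to EnemyEffects_1, which has no handler yet.
; Refresh resets mana, fills the hand from the top of the deck and prints debug names.
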(event EventBeginPlay
  (Variables|Default|SetbIsStateDone false)
  (CallFunction|ExecuteStartGame)
  (Variables|Default|SetState "NewEnumerator0")
  (Development|PrintString "AAAAAAAAAAAAAAAAAAAA"))

(event EventTick
  (params (DeltaSeconds :type Float%20%28single-precision%29))
  (if (Variables|Default|GetbIsStateDone)
    (switch Utilities|FlowControl|Switch|SwitchonGameStates (Variables|Default|GetState)
      (:NewEnumerator0
        (Variables|Default|SetbIsStateDone false)
        (CallFunction|ExecuteRefresh)
        (Variables|Default|SetbIsStateDone true)
        (Variables|Default|SetState "NewEnumerator1")))
    (else
      (CallFunction|ExecuteRefresh)
      (Variables|Default|SetbIsStateDone true))))

(fn ConstructionScript)

(fn ExecuteRefresh
  (bind _handlist (Variables|Default|GetHandList))
  (Variables|Default|SetMana 5)
  (Development|PrintString "Hello")
  (bind _output_get (LocalVariables|SetCards%20To%20Draw (- (- 5 (Utilities|Array|Length (Variables|Default|GetHandList))) 1)))
  ;[0.15 0.15 0.15 0.5] Draw from deck
  (for _index (range 0 _output_get)
    (bind _returnvalue (Utilities|Array|Add _handlist (Utilities|Array|Get(acopy) (Variables|Default|GetDeckList) _index)))
    (Development|PrintString (Utilities|GetDisplayName (Utilities|Array|Get(acopy) _handlist _returnvalue)) true true "(R=0.000000,G=0.660000,B=1.000000,A=1.000000)" 1e+02))
  ;[0.15 0.15 0.15 0.5] Remove drawn cards from deck
  (for _index_2 (range 0 _output_get)
    (Development|PrintString (Utilities|GetDisplayName (Utilities|Array|Get(acopy) (Variables|Default|GetDeckList))) true true "(R=0.000000,G=0.660000,B=1.000000,A=1.000000)" 1e+02)
    (Utilities|Array|RemoveIndex (Variables|Default|GetDeckList))))

(fn ExecuteStartGame
  (bind _outactors (Actor|GetAllActorsOfClass "/Game/Blueprint/Card/BP_DummyCard.BP_DummyCard_C"))
  (bind _output_get (Variables|Default|SetDeckList _outactors))
  (Utilities|Array|Shuffle _output_get)
  (for _array_element _output_get
    _))