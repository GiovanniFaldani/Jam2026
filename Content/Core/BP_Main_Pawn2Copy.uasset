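; Player pawn for a turn-based card game that routes mouse and pass input according to the GameMode's state.
; Cursor traces drive interface-based card clicks in Play, plus clicks, right-clicks and dragging in Deck Building; other phases play click sounds.
; Tick updates drags, runs a placeholder delayed effects phase, and on entering Play flags hand cards interactable by mana cost.
; Passing ends Play by switching to Count.
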(event Input|EnhancedActionEvents|EnhancedInputActionIA_LMouseDown
  (params (ActionValue :type Boolean) (ElapsedSeconds :type Float%20%28double-precision%29) (TriggeredSeconds :type Float%20%28double-precision%29) (InputAction :type Input%20Action%20Object%20Reference :default "/Game/Input/InputAction/IA_LMouseDown.IA_LMouseDown"))
  (bind _asbp_main_game_mode (Utilities|Casting|CastToBP_Main_GameMode (Game|GetGameMode)))
  (switch Utilities|FlowControl|Switch|SwitchonGameStates (Variables|/Game/Core/BP_Main_GameMode.BP_Main_GameMode_C|GetState _asbp_main_game_mode)
    (:NewEnumerator9
      (CallFunction|CheckDrag))))

(event Input|EnhancedActionEvents|EnhancedInputActionIA_LMouseClick
  (params (ActionValue :type Boolean) (ElapsedSeconds :type Float%20%28double-precision%29) (TriggeredSeconds :type Float%20%28double-precision%29) (InputAction :type Input%20Action%20Object%20Reference :default "/Game/Input/InputAction/IA_LMouseClick.IA_LMouseClick"))
  (bind _asbp_main_game_mode (Utilities|Casting|CastToBP_Main_GameMode (Game|GetGameMode)))
  (switch Utilities|FlowControl|Switch|SwitchonGameStates (Variables|/Game/Core/BP_Main_GameMode.BP_Main_GameMode_C|GetState _asbp_main_game_mode)
    (:NewEnumerator0
      (Audio|PlaySound2D "/Game/sounds/SFX/TURN_START_SFX.TURN_START_SFX" 1.0 1.0 0.0 0 0))
    (:NewEnumerator1
      (Audio|PlaySound2D "/Game/sounds/SFX/ENEMY_ABILITY_SFX.ENEMY_ABILITY_SFX" 1.0 1.0 0.0 0 0))
    (:NewEnumerator3
      (CallFunction|ClickinPlay))
    (:NewEnumerator7
      (Audio|PlaySound2D "/Game/sounds/SFX/DAMAGE_SFX.DAMAGE_SFX" 1.0 1.0 0.0 0 0))
    (:NewEnumerator9
      (CallFunction|CheckMask))))

(event Input|EnhancedActionEvents|EnhancedInputActionIA_LMouseUp
  (params (ActionValue :type Boolean) (ElapsedSeconds :type Float%20%28double-precision%29) (TriggeredSeconds :type Float%20%28double-precision%29) (InputAction :type Input%20Action%20Object%20Reference :default "/Game/Input/InputAction/IA_LMouseUp.IA_LMouseUp"))
  (bind _asbp_main_game_mode (Utilities|Casting|CastToBP_Main_GameMode (Game|GetGameMode)))
  (switch Utilities|FlowControl|Switch|SwitchonGameStates (Variables|/Game/Core/BP_Main_GameMode.BP_Main_GameMode_C|GetState _asbp_main_game_mode)
    (:NewEnumerator9
      (if (Variables|Default|GetbIsDragging)
        (if (Utilities|IsValidInterface (Variables|Default|GetDraggedObject))
          (Variables|Default|SetbIsDragging false)
          (Default|EndDrag (Variables|Default|GetDraggedObject)))))))

(event Input|EnhancedActionEvents|EnhancedInputActionIA_RMouseClick
  (params (ActionValue :type Boolean) (ElapsedSeconds :type Float%20%28double-precision%29) (TriggeredSeconds :type Float%20%28double-precision%29) (InputAction :type Input%20Action%20Object%20Reference :default "/Game/Input/InputAction/IA_RMouseClick.IA_RMouseClick"))
  (bind _asbp_main_game_mode (Utilities|Casting|CastToBP_Main_GameMode (Game|GetGameMode)))
  (switch Utilities|FlowControl|Switch|SwitchonGameStates (Variables|/Game/Core/BP_Main_GameMode.BP_Main_GameMode_C|GetState _asbp_main_game_mode)
    (:NewEnumerator9
      (CallFunction|CheckCard))))

(event Input|EnhancedActionEvents|EnhancedInputActionIA_Pass
  (params (ActionValue :type Boolean) (ElapsedSeconds :type Float%20%28double-precision%29) (TriggeredSeconds :type Float%20%28double-precision%29) (InputAction :type Input%20Action%20Object%20Reference :default "/Game/Input/InputAction/IA_Pass.IA_Pass"))
  (bind _asbp_main_game_mode (Utilities|Casting|CastToBP_Main_GameMode (Game|GetGameMode)))
  (switch Utilities|FlowControl|Switch|SwitchonGameStates (Variables|/Game/Core/BP_Main_GameMode.BP_Main_GameMode_C|GetState _asbp_main_game_mode)
    (:NewEnumerator3
      (Variables|/Game/Core/BP_Main_GameMode.BP_Main_GameMode_C|SetbIsStateDone _asbp_main_game_mode true)
      (Variables|Default|SetbStartPlay true)
      (Variables|/Game/Core/BP_Main_GameMode.BP_Main_GameMode_C|SetState _asbp_main_game_mode "NewEnumerator4"))))

(event EventBeginPlay)

(event Collision|EventActorBeginOverlap
  (params (OtherActor :type Actor%20Object%20Reference)))

(event EventTick
  (params (DeltaSeconds :type Float%20%28single-precision%29))
  (bind _asbp_main_game_mode (Utilities|Casting|CastToBP_Main_GameMode (Game|GetGameMode)))
  (switch Utilities|FlowControl|Switch|SwitchonGameStates (Variables|/Game/Core/BP_Main_GameMode.BP_Main_GameMode_C|GetState _asbp_main_game_mode)
    (:NewEnumerator2
      (Variables|/Game/Core/BP_Main_GameMode.BP_Main_GameMode_C|SetbIsStateDone _asbp_main_game_mode false)
      ;[0.15 0.15 0.15 0.5] TODO animation and effects
      (Development|PrintString "Hello from enemy" true true "(R=0.000000,G=0.660000,B=1.000000,A=1.000000)" 2.0 "Enemy")
      (Utilities|FlowControl|Delay 2.0)
      (Variables|/Game/Core/BP_Main_GameMode.BP_Main_GameMode_C|SetbIsStateDone _asbp_main_game_mode true)
      (Variables|/Game/Core/BP_Main_GameMode.BP_Main_GameMode_C|SetState _asbp_main_game_mode "NewEnumerator3"))
    (:NewEnumerator3
      (Variables|/Game/Core/BP_Main_GameMode.BP_Main_GameMode_C|SetbIsStateDone _asbp_main_game_mode false)
      (CallFunction|ExecutePlay))
    (:NewEnumerator9
      (if (Variables|Default|GetbIsDragging)
        (Default|Drag (Variables|Default|GetDraggedObject))))))

(event EventPossessed
  (params (NewController :type Controller%20Object%20Reference))
  (bind _asbp_main_player_controller (Utilities|Casting|CastToBP_Main_PlayerController (Pawn|GetController)))
  (Input|AddMappingContext (PlayerController|LocalPlayerSubsystems|GetEnhancedInputLocalPlayerSubsystem _asbp_main_player_controller) "/Game/Input/IMC_MouseControls.IMC_MouseControls" 0 "(bIgnoreAllPressedKeysUntilRelease=True,bForceImmediately=False,bNotifyUserSettings=False)"))

(fn ConstructionScript)

(fn CheckDrag
  (bind _returnvalue (Game|GetPlayerController 0))
  (bind (_hitresult _returnvalue_2) (Game|Player|GetHitResultUnderCursorbyChannel _returnvalue "TraceTypeQuery3" true))
  (if _returnvalue_2
    (bind _asbpi_draggable (Utilities|Casting|CastToBPI_Draggable (.HitActor (Collision|BreakHitResult _hitresult))))
    (Variables|Default|SetDraggedObject _asbpi_draggable)
    (Variables|Default|SetbIsDragging true)))

(fn CheckMask
  (bind _returnvalue (Game|GetPlayerController 0))
  (bind (_hitresult _returnvalue_2) (Game|Player|GetHitResultUnderCursorbyChannel _returnvalue "TraceTypeQuery4" true))
  (if _returnvalue_2
    (bind _asbpi_clickable (Utilities|Casting|CastToBPI_Clickable (.HitActor (Collision|BreakHitResult _hitresult))))
    (Default|Click _asbpi_clickable)))

(fn CheckCard
  (bind _returnvalue (Game|GetPlayerController 0))
  (bind (_hitresult _returnvalue_2) (Game|Player|GetHitResultUnderCursorbyChannel _returnvalue "TraceTypeQuery4" true))
  (if _returnvalue_2
    (bind _asbpi_clickable (Utilities|Casting|CastToBPI_Clickable (.HitActor (Collision|BreakHitResult _hitresult))))
    (Default|RClick _asbpi_clickable)))

(fn ExecutePlay
  ;[0.15 0.15 0.15 0.5] TODO post init
  (if (Variables|Default|GetbStartPlay)
    (if true
      (bind _asbp_main_game_mode (Utilities|Casting|CastToBP_Main_GameMode (Game|GetGameMode)))
      (for _array_element (Variables|/Game/Core/BP_Main_GameMode.BP_Main_GameMode_C|GetHandList _asbp_main_game_mode)
        (if (>= (Variables|/Game/Core/BP_Main_GameMode.BP_Main_GameMode_C|GetMana _asbp_main_game_mode) (Variables|/Game/Blueprint/Card/BP_DummyCard.BP_DummyCard_C|GetCost _array_element))
          (Variables|/Game/Blueprint/Card/BP_DummyCard.BP_DummyCard_C|SetbIsInteractable _array_element true)
          (Development|PrintString "Interactable" true true "(R=0.000000,G=1.000000,B=0.134542,A=1.000000)" 1e+01 "")
          (else
            (Variables|/Game/Blueprint/Card/BP_DummyCard.BP_DummyCard_C|SetbIsInteractable _array_element false)
            (Development|PrintString "Non Interactable" true true "(R=0.000000,G=1.000000,B=0.134542,A=1.000000)" 1e+01 ""))))
      (Variables|Default|SetbStartPlay false))))

(fn ClickinPlay
  (bind _returnvalue (Game|GetPlayerController 0))
  (bind (_hitresult _returnvalue_2) (Game|Player|GetHitResultUnderCursorbyChannel _returnvalue "TraceTypeQuery4" true))
  (if _returnvalue_2
    (bind _asbpi_clickable (Utilities|Casting|CastToBPI_Clickable (.HitActor (Collision|BreakHitResult _hitresult))))
    (Default|Click _asbpi_clickable)))