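; BP_EnemyTut is an enemy actor whose skeletal mesh animations follow the turn state of BP_Main_GameMode.
; On BeginPlay it plays an entrance animation, then switches to looping idle after a delay.
; Tick polls the game mode and, during Enemy Effects 1, calls the attack animation every frame without a guard, with a delayed return to idle.
; The construction script snaps a static mesh to the "Faccia" socket.
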(event EventBeginPlay
  (|CallParentFunction)
  (Components|Animation|PlayAnimation (Variables|Default|GetAnimazioni_finite) "/Game/Assets/Models/Boss/Animazioni_finite_Anim_entro_in_scena.Animazioni_finite_Anim_entro_in_scena" false)
  (Utilities|FlowControl|Delay 3.0)
  (Components|Animation|PlayAnimation (Variables|Default|GetAnimazioni_finite) "/Game/Assets/Models/Boss/Animazioni_finite_Anim_idle.Animazioni_finite_Anim_idle" true))

(event Collision|EventActorBeginOverlap
  (params (OtherActor :type Actor%20Object%20Reference))
  (|CallParentFunction OtherActor) ; This node is disabled and will not be called.\nDrag off pins to build functionality.
)

(event EventTick
  (params (DeltaSeconds :type Float%20%28single-precision%29))
  (|CallParentFunction DeltaSeconds)
  (bind _asbp_main_game_mode (Utilities|Casting|CastToBP_Main_GameMode (Game|GetGameMode)))
  (switch Utilities|FlowControl|Switch|SwitchonGameStates (Variables|/Game/Core/BP_Main_GameMode.BP_Main_GameMode_C|GetState _asbp_main_game_mode)
    (:NewEnumerator1
      (Components|Animation|PlayAnimation (Variables|Default|GetAnimazioni_finite) "/Game/Assets/Models/Boss/Animazioni_finite_Anim_attacco_migliorato_001.Animazioni_finite_Anim_attacco_migliorato_001" false)
      (Utilities|FlowControl|Delay 5.0)
      (Components|Animation|PlayAnimation (Variables|Default|GetAnimazioni_finite) "/Game/Assets/Models/Boss/Animazioni_finite_Anim_idle.Animazioni_finite_Anim_idle" true))))

(fn ConstructionScript
  (|CallParentFunction)
  (Transformation|AttachComponentToComponent (Variables|Default|GetStaticMesh) (Variables|Default|GetAnimazioni_finite) "Faccia" "SnapToTarget" "SnapToTarget" "SnapToTarget" true))