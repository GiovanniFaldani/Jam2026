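; BP_DummyCard is a playable card actor that loads its cost, value, name and effect tags from a data table row at construction.
; Clicking an interactable card moves it from hand to play in BP_Main_GameMode, spends mana, adds turn value, flags the pawn and re-lays out cards.
; Mask gameplay tags swap the card material, and right-click during deck building applies NoMask.
; Effect tags are not yet applied on play (TODO).
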(event EventBeginPlay)

(event Collision|EventActorBeginOverlap
  (params (OtherActor :type Actor%20Object%20Reference)))

(event EventTick
  (params (DeltaSeconds :type Float%20%28single-precision%29)))

(event EventClick
  (bind _self self)
  (if (Variables|Default|GetbIsInteractable)
    (bind _asbp_main_game_mode (Utilities|Casting|CastToBP_Main_GameMode (Game|GetGameMode)))
    (Utilities|Array|AddUnique (Variables|/Game/Core/BP_Main_GameMode.BP_Main_GameMode_C|GetPlayList _asbp_main_game_mode) _self)
    (Utilities|Array|RemoveItem (Variables|/Game/Core/BP_Main_GameMode.BP_Main_GameMode_C|GetHandList _asbp_main_game_mode) _self)
    (Variables|Default|SetbIsInteractable false)
    (Variables|/Game/Core/BP_Main_GameMode.BP_Main_GameMode_C|SetMana _asbp_main_game_mode (- (Variables|/Game/Core/BP_Main_GameMode.BP_Main_GameMode_C|GetMana _asbp_main_game_mode) (Variables|Default|GetCost)))
    ;[0.15 0.15 0.15 0.5] TODO aggiungi effetti a tag
    (Variables|/Game/Core/BP_Main_GameMode.BP_Main_GameMode_C|SetTurnValue _asbp_main_game_mode (+ (Variables|/Game/Core/BP_Main_GameMode.BP_Main_GameMode_C|GetTurnValue _asbp_main_game_mode) (Variables|Default|GetValue)))
    (bind _asbp_main_pawn_1 (Utilities|Casting|CastToBP_Main_Pawn1 (Pawn|GetControlledPawn (Game|GetPlayerController 0))))
    (Variables|/Game/Core/BP_Main_Pawn1.BP_Main_Pawn1_C|SetbStartPlay _asbp_main_pawn_1 true)
    (Rendering|Material|SetMaterial (Variables|Default|GetCardBaseMesh) 0 "/Game/Materials/Instances/MI_Yellow.MI_Yellow")
    (Default|MoveCardsinHand _asbp_main_game_mode)
    (Default|MoveCardsinPlay _asbp_main_game_mode)
    (else
      (Development|PrintString "Card not playable" true true "(R=0.000000,G=0.660000,B=1.000000,A=1.000000)" 2.0 "Card"))))

(event EventAddModifier
  (params (MaskType :type Gameplay%20Tag%20Structure))
  (|SwitchGameplayTag MaskType
    (:Default
      (Rendering|Material|SetMaterial (Variables|Default|GetCardBaseMesh) 0 "/Game/Materials/Instances/MI_White.MI_White"))
    (:MaskType.Dummy
      (Rendering|Material|SetMaterial (Variables|Default|GetCardBaseMesh) 0 "/Game/Materials/Instances/MI_Red.MI_Red"))))

(event EventRClick
  (bind _asbp_main_game_mode (Utilities|Casting|CastToBP_Main_GameMode (Game|GetGameMode)))
  (switch Utilities|FlowControl|Switch|SwitchonGameStates (Variables|/Game/Core/BP_Main_GameMode.BP_Main_GameMode_C|GetState _asbp_main_game_mode)
    (:NewEnumerator9
      (CallFunction|AddModifier "(TagName=\"MaskType.NoMask\")"))))

(fn ConstructionScript
  (CallFunction|LoadData))

(fn LoadData
  (bind _rowname (Variables|Default|GetRowName))
  (bind _returnvalue (Utilities|GetDataTableRow "/Game/Blueprint/Data/CardDatas.CardDatas" _rowname)
    (:then
      (Variables|Default|SetCost (.cost _returnvalue))
      (Variables|Default|SetValue (.value _returnvalue))
      (Variables|Default|SetEffect%20Tags (.maskeffects _returnvalue))
      (Variables|Default|SetName (.cardname _returnvalue)))
    (:RowNotFound
      (Development|PrintString (Utilities|String|ToString(Name) _rowname)))))