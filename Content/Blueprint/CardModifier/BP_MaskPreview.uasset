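; BP_MaskPreview is a draggable preview of a mask that applies a card modifier when dropped on a card.
; Init sets the sphere component's mesh and material and stores the mask tag.
; Drag follows the deprojected mouse position in X and Y while keeping its height.
; EndDrag traces under the cursor, passes the tag to AddModifier on any BP_DummyCard hit, and destroys the preview in every case.
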(event EventBeginPlay)

(event Collision|EventActorBeginOverlap
  (params (OtherActor :type Actor%20Object%20Reference)))

(event EventTick
  (params (DeltaSeconds :type Float%20%28single-precision%29)))

(event EventDrag
  (bind _returnvalue (Game|GetPlayerController 0))
  (bind _worldlocation (Game|Player|ConvertMouseLocationToWorldSpace _returnvalue))
  (Development|PrintString "Dragging..." true true "(R=1.000000,G=0.000000,B=0.000000,A=1.000000)" 0.1 "Drag")
  (Transformation|SetActorLocation (Math|Vector|MakeVector (.x _worldlocation) (.y _worldlocation) (.z (Transformation|GetActorLocation self))) false false))

(event EventEndDrag
  (bind _returnvalue (Game|GetPlayerController 0))
  (bind (_hitresult _returnvalue_2) (Game|Player|GetHitResultUnderCursorbyChannel _returnvalue "TraceTypeQuery1" true))
  (Development|PrintString "End drag" true true "(R=1.000000,G=0.000000,B=0.000000,A=1.000000)" 0.5 "Drag")
  (if _returnvalue_2
    (bind _asbp_dummy_card (Utilities|Casting|CastToBP_DummyCard (.HitActor (Collision|BreakHitResult _hitresult)))
      (:then
        (Default|AddModifier _asbp_dummy_card (Variables|Default|GetPreviewMaskTag))
        (Actor|DestroyActor))
      (:CastFailed
        (Actor|DestroyActor)))
    (else
      (Actor|DestroyActor))))

(fn ConstructionScript)

(fn Init
  (params (NewMesh :type Static%20Mesh%20Object%20Reference) (NewMaskType :type Gameplay%20Tag%20Structure))
  (Rendering|Material|SetMaterial (Variables|Default|GetSphere) 0 (Rendering|Material|GetMaterial NewMesh 0))
  (Components|StaticMesh|SetStaticMesh (Variables|Default|GetSphere) NewMesh)
  (Variables|Default|SetPreviewMaskTag NewMaskType))