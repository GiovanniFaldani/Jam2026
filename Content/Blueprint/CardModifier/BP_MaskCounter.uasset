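; Actor that tracks how many masks of each type remain available, likely as card modifiers.
; On BeginPlay it fills a counter map from the mask tag list, giving every type the same starting count.
; TryUseMask decrements the matching count, or prints an on-screen warning when none are left.
; CheckMaskDraggable reports whether a type still has masks remaining, as a test for whether it can be dragged.
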(event EventBeginPlay
  (for _array_element (Variables|Default|GetMaskTagList)
    (Utilities|Map|Add (Variables|Default|GetMask%20Counter%20Map) _array_element (Variables|Default|GetStartingMasksPerType))))

(event Collision|EventActorBeginOverlap
  (params (OtherActor :type Actor%20Object%20Reference)))

(event EventTick
  (params (DeltaSeconds :type Float%20%28single-precision%29)))

(fn ConstructionScript)

(fn TryUseMask
  (params (Mask%20Type :type Gameplay%20Tag%20Structure))
  (bind _mask_counter_map (Variables|Default|GetMask%20Counter%20Map))
  (bind _value (Utilities|Map|Find _mask_counter_map Mask%20Type))
  (if (> _value 0)
    (Utilities|Map|Add _mask_counter_map Mask%20Type (- _value 1))
    (else
      (Development|PrintString "Not enough masks!" true true "(R=1.000000,G=0.000000,B=0.316242,A=1.000000)" 2.0 "MaskCount"))))

(fn CheckMaskDraggable
  (params (MaskType :type Gameplay%20Tag%20Structure))
  (return (> (.Value (Utilities|Map|Find (Variables|Default|GetMask%20Counter%20Map) MaskType)) 0)))