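; BP_Mask is a clickable card-modifier mask actor identified by a MaskType gameplay tag.
; Clicking it spawns a BP_MaskPreview just above the mask at the same rotation and scale, initialized with the mask's static mesh and type.
; BeginPlay switches on MaskType under a "Set mask asset" comment, but no branch logic follows.
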(event EventBeginPlay
  ;[0.15 0.15 0.15 0.5] Set mask asset
  (|SwitchGameplayTag (Variables|Default|GetMaskType)))

(event Collision|EventActorBeginOverlap
  (params (OtherActor :type Actor%20Object%20Reference)))

(event EventTick
  (params (DeltaSeconds :type Float%20%28single-precision%29)))

(event EventClick
  (CallFunction|SpawnPreview))

(fn ConstructionScript)

(fn SpawnPreview
  (bind _returnvalue (Transformation|GetActorTransform))
  (bind _output_get (LocalVariables|SetSpawnTransform (Math|Transform|MakeTransform (Math|Vector|MakeVector (.x (.location _returnvalue)) (.y (.location _returnvalue)) (+ (.z (.location _returnvalue)) 0.1)) (.rotation _returnvalue) (.scale _returnvalue))))
  (bind _returnvalue_2 (Game|SpawnActorfromClass "/Game/Blueprint/CardModifier/BP_MaskPreview.BP_MaskPreview_C" _output_get "Undefined" "MultiplyWithRoot" 0 0))
  (Default|Init _returnvalue_2 (Variables|/Script/Engine.StaticMeshComponent|GetStaticMesh (Variables|Default|GetMesh)) (Variables|Default|GetMaskType)))